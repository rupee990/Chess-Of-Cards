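; BP_RandomCard is an actor that spawns a MyCard just above itself when its Box is clicked.
; The new card gets a row handle into DT_CardsTable from this actor's RowName, then its paper sprite is set from that row.
; No random selection happens in this Blueprint, despite the name.
; A separate DEstroy function removes the actor and is not called here.
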(event `self.Box.OnClicked`
  (params (TouchedComponent :type "PrimitiveComponent Object Reference") (ButtonPressed :type "Key Structure"))
  (bind _returnvalue (`|SpawnActorFromClass` "/Game/PuzzleCPP/MyCard.MyCard_C" (`KismetMathLibrary.Conv_VectorToTransform` (`KismetMathLibrary.MakeVector` (.x (`self.K2_GetActorLocation`)) (.y (`self.K2_GetActorLocation`)) (+ (.z (`self.K2_GetActorLocation`)) 100.0))) "Undefined" "OverrideRootScale" null null))
  (bind _asmy_card (cast `/Game/PuzzleCPP/MyCard` _returnvalue))
  (bind _output_get (set `Card.m_RowHandle` (make `DataTableRowHandle` "/Game/PuzzleCPP/DT_CardsTable.DT_CardsTable" (`self.RowName`)) _asmy_card))
  (bind (_datatable _rowname) (break `DataTableRowHandle` _output_get))
  (bind _returnvalue_2 (`|GetDataTableRow` _datatable _rowname)
    (:`then`
      (`PaperSpriteComponent.SetSprite` (`Card.m_PaperSpriteComponent` _asmy_card) (`.m_Sprite` (break `CardData` _returnvalue_2))))))

(fn `DEstroy`
  (`self.K2_DestroyActor`))

(fn `UserConstructionScript`)