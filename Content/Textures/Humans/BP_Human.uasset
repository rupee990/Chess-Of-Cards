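; BP_Human is a randomly generated sprite-based person, built on BeginPlay, who comes with an ID card.
; GenerateHuman picks hair, head and body sprites from data tables, randomly tinting parts whose rows allow it.
; It rolls a first name and adult age, but assigns fixed insignia sprites.
; It destroys any existing card, then spawns a BP_IdCard at CardDrop with these details and links it back to the human.
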(event `self.ReceiveBeginPlay`
  (`self.GenerateHuman`))

(fn `GenerateHuman`
  (bind _hair (`self.Hair`))
  (bind _head (`self.Head`))
  (`/Engine/EditorBlueprintResources/StandardMacros.IsValid` (`self.Card_Id`)
    (:`Is Valid`
      (`Card.DestroyCard` (`self.Card_Id`)))
    (:`Is Not Valid`
      _))
  (`|ExecutionSequence`
    (:`then_0`
      ;[1 1 1] Set Hairs
      (bind _rowdata (`self.GetRandomDataTableEntry` (`self.HairsTable`)))
      (bind (_sprite _getrandomcolor) (break `/Game/Textures/Humans/SpriteStruct` _rowdata))
      (`PaperSpriteComponent.SetSprite` _hair _sprite)
      (if _getrandomcolor
        (`PaperSpriteComponent.SetSpriteColor` _hair (`self.RandomColor`))))
    (:`then_1`
      ;[1 1 1] Set Head
      (bind _rowdata_2 (`self.GetRandomDataTableEntry` (`self.HeadTable`)))
      (bind (_sprite_2 _getrandomcolor_2) (break `/Game/Textures/Humans/SpriteStruct` _rowdata_2))
      (`PaperSpriteComponent.SetSprite` _head _sprite_2)
      (if _getrandomcolor_2
        (`PaperSpriteComponent.SetSpriteColor` _head (`self.RandomColor`))))
    (:`then_2`
      ;[1 1 1] Set Body
      (bind _rowdata_3 (`self.GetRandomDataTableEntry` (`self.BodyTable`)))
      (bind (_sprite_3 _getrandomcolor_3) (break `/Game/Textures/Humans/SpriteStruct` _rowdata_3))
      (`PaperSpriteComponent.SetSprite` (`self.Body`) _sprite_3)
      (if _getrandomcolor_3
        (`PaperSpriteComponent.SetSpriteColor` (`self.Body`) (`self.RandomColor`))))
    (:`then_3`
      (bind _rowentry (`self.GetRandomRow` "/Game/Textures/Humans/DT_FirstNames.DT_FirstNames")
        (:`OutExec`
          (set `self.Name` (`KismetStringLibrary.Conv_StringToName` (`.Name_6_DEA1FC0D4B02E6DBBD69F4AC7FFB9816` (break `/Game/Textures/Humans/S_Names` _rowentry))))
          (set `self.Age` (`KismetMathLibrary.RandomIntegerInRange` 21 75))
          (set `self.Class` "/Game/Textures/Humans/Insignias_Sprite_0.Insignias_Sprite_0")
          (set `self.CityInsignia` "/Game/Textures/Humans/Insignias_Sprite_3.Insignias_Sprite_3")
          (set `self.CitizenInsignia` "/Game/Textures/Humans/Insignias_Sprite_2.Insignias_Sprite_2"))))
    (:`then_4`
      (bind _returnvalue (`|SpawnActorFromClass` "/Game/Textures/Humans/BP_IdCard.BP_IdCard_C" (`KismetMathLibrary.Conv_VectorToTransform` (`SceneComponent.K2_GetComponentLocation` (`self.CardDrop`))) "Undefined" "OverrideRootScale" null (`self.Name`) (`self.Age`) (`self.CitizenInsignia`) (`self.CityInsignia`) (`self.Class`) null))
      (bind _output_get (set `self.Card_Id` _returnvalue))
      (set `/Game/Textures/Humans/BP_IdCard.HumanRef` self _output_get)
      (`/Game/Textures/Humans/BP_IdCard.SetCardInfo` _returnvalue))))

(fn `GetRandomDataTableEntry`
  (params (DataTable :type "DataTable Object Reference"))
  (returns (RowData :type "/Game/Textures/Humans/SpriteStruct Structure"))
  (bind _outrownames (`DataTableFunctionLibrary.GetDataTableRowNames` DataTable))
  (bind _returnvalue (`|GetDataTableRow` DataTable (`self.GetRandomArrayEntry` _outrownames))
    (:`then`
      (return _returnvalue))))

(fn `UserConstructionScript`)