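; BP_IdCard is an ID card that shows a human's portrait and identity details.
; Its SetCardInfo event copies hair, head and body sprites and colors from the referenced human into the card's own sprite components.
; It also fills the city insignia, citizen insignia and class sprites, plus name and age text, from the card's variables.
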(event `SetCardInfo`
  (bind _hair (`self.Hair`))
  (bind _head (`self.Head`))
  (bind _body (`self.Body`))
  (bind _hair_2 (`/Game/Textures/Humans/BP_Human.Hair` (`self.HumanRef`)))
  (bind _head_2 (`/Game/Textures/Humans/BP_Human.Head` (`self.HumanRef`)))
  (bind _body_2 (`/Game/Textures/Humans/BP_Human.Body` (`self.HumanRef`)))
  (`PaperSpriteComponent.SetSprite` _hair (`PaperSpriteComponent.GetSprite` _hair_2))
  (`PaperSpriteComponent.SetSpriteColor` _hair (`PaperSpriteComponent.SpriteColor` _hair_2))
  (`PaperSpriteComponent.SetSprite` _head (`PaperSpriteComponent.GetSprite` _head_2))
  (`PaperSpriteComponent.SetSpriteColor` _head (`PaperSpriteComponent.SpriteColor` _head_2))
  (`PaperSpriteComponent.SetSprite` _body (`PaperSpriteComponent.GetSprite` _body_2))
  (`PaperSpriteComponent.SetSpriteColor` _body (`PaperSpriteComponent.SpriteColor` _body_2))
  (`PaperSpriteComponent.SetSprite` (`self.CityInsignia`) (`self.CityInsSprite`))
  (`PaperSpriteComponent.SetSprite` (`self.CitizenInsignia`) (`self.CitizenInsSprite`))
  (`PaperSpriteComponent.SetSprite` (`self.Class`) (`self.ClassValue`))
  (`TextRenderComponent.K2_SetText` (`self.NameValue`) (`KismetTextLibrary.Conv_NameToText` (`self.Name`)))
  (`TextRenderComponent.K2_SetText` (`self.AgeValue`) (`KismetTextLibrary.Conv_IntToText` (`self.Age`))))

(fn `UserConstructionScript`)