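; BP_PlayerView is the puzzle's camera view and mouse controller for dragging cards onto board spaces to place pieces.
; On begin play it becomes the view target and enables the cursor and click events.
; Visibility traces from the camera through the cursor pick up a MyCard and move it each tick at a fixed height.
; Releasing over a board space spawns a StaticMeshActor using the card's data table mesh and material, then destroys the card.
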(event `self.ReceiveBeginPlay`
  (bind _returnvalue (`GameplayStatics.GetPlayerController` 0))
  (`PlayerController.SetViewTargetWithBlend` _returnvalue self 0.0 "VTBlend_Linear" 0.0 false)
  (set `PlayerController.bEnableClickEvents` true _returnvalue)
  (set `PlayerController.bShowMouseCursor` true _returnvalue))

(event `self.ReceiveTick`
  (params (DeltaSeconds :type "Float (single-precision)"))
  (bind _grabbed_card (`self.Grabbed_Card`))
  (bind (_worldlocation _worlddirection) (`PlayerController.DeprojectMousePositionToWorld` (`GameplayStatics.GetPlayerController` 0)))
  (`/Engine/EditorBlueprintResources/StandardMacros.IsValid` _grabbed_card
    (:`Is Valid`
      (bind (_outhit _returnvalue) (`KismetSystemLibrary.LineTraceSingle` (`SceneComponent.K2_GetComponentLocation` (`self.Camera`)) (+ _worldlocation (* _worlddirection 10000.0)) "TraceTypeQuery1"))
      (if _returnvalue
        (bind (_bblockinghit _binitialoverlap _time _distance _location _impactpoint) (`GameplayStatics.BreakHitResult` _outhit))
        (`self.K2_SetActorLocation` _grabbed_card (`KismetMathLibrary.MakeVector` (.x _impactpoint) (.y _impactpoint) 100.0) false false)))))

(event `InputAction|MouseGrab`
  (params (Key :type "Key Structure"))
  (bind _grabbed_card (`self.Grabbed_Card`))
  (bind _grabbed_card_2 (`self.Grabbed_Card`))
  (bind (_worldlocation _worlddirection) (`PlayerController.DeprojectMousePositionToWorld` (`GameplayStatics.GetPlayerController` 0)))
  (bind _m_boardspace (`Card.m_BoardSpace` _grabbed_card))
  (bind (_datatable _rowname) (break `DataTableRowHandle` (`Card.m_RowHandle` _grabbed_card)))
  (:`Pressed`
    (bind _outhit (`KismetSystemLibrary.LineTraceSingle` :`Start` (`SceneComponent.K2_GetComponentLocation` (`self.Camera`)) :`End` (+ _worldlocation (* _worlddirection 10000.0)) :`TraceChannel` "TraceTypeQuery1" :`DrawTime` 10.0))
    (bind _asmy_card (cast `/Game/PuzzleCPP/MyCard` (`.HitActor` (`GameplayStatics.BreakHitResult` _outhit))))
    (set `self.Grabbed_Card` _asmy_card))
  (:`Released`
    (`/Engine/EditorBlueprintResources/StandardMacros.IsValid` _grabbed_card
      (:`Is Valid`
        (`/Engine/EditorBlueprintResources/StandardMacros.IsValid` _m_boardspace
          (:`Is Valid`
            (bind _returnvalue (`|GetDataTableRow` _datatable _rowname)
              (:`then`
                (bind _returnvalue_2 (`|SpawnActorFromClass` "/Script/Engine.StaticMeshActor" (`KismetMathLibrary.Conv_VectorToTransform` (`KismetMathLibrary.MakeVector` (.x (`self.K2_GetActorLocation` _m_boardspace)) (.y (`self.K2_GetActorLocation` _m_boardspace)) (+ (.z (`self.K2_GetActorLocation` _m_boardspace)) 50.0))) "Undefined" "OverrideRootScale" null null))
                (`StaticMeshActor.SetMobility` _returnvalue_2 "Movable")
                (bind _staticmeshcomponent (`StaticMeshActor.StaticMeshComponent` _returnvalue_2))
                (bind (_m_sprite _m_piecemesh _m_piecematerial) (break `CardData` _returnvalue))
                (`StaticMeshComponent.SetStaticMesh` _staticmeshcomponent _m_piecemesh)
                (`PrimitiveComponent.SetMaterial` _staticmeshcomponent 0 _m_piecematerial)
                (set `Card.m_BoardSpace` null _grabbed_card_2)
                (`Card.DestroyCard` _grabbed_card_2))))
          (:`Is Not Valid`
            _))
        (set `self.Grabbed_Card` null)))))

(fn `UserConstructionScript`)